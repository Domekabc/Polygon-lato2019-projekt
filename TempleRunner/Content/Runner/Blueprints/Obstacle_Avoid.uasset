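; Obstacle actor for the runner game that kills the player's ThirdPersonCharacter on overlap.
; The construction script randomly dresses the Pipe mesh component as a box, rock or round table, adjusting world scale and rotation for the latter two.
; On actor overlap, it casts to the character and calls its DeathFunction through a DoOnce, so the death triggers only once per obstacle.
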(event `self.ReceiveActorBeginOverlap`
  (params (OtherActor :type "Actor Object Reference"))
  (bind _asthird_person_character (cast `/Game/ThirdPersonBP/ThirdPersonCharacter` OtherActor))
  (`/Engine/EditorBlueprintResources/StandardMacros.DoOnce` false
    (:`Completed`
      (`/Game/ThirdPersonBP/ThirdPersonCharacter.DeathFunction` _asthird_person_character))))

(fn `UserConstructionScript`
  (bind _pipe (`self.Pipe`))
  (bind _pipe_2 (`self.Pipe`))
  (switch `int` (`KismetMathLibrary.RandomInteger` 3)
    (:`0`
      ;[1 1 1] Box
      (`StaticMeshComponent.SetStaticMesh` (`self.Pipe`) "/Game/Runner/Meshes/box.box"))
    (:`1`
      ;[1 1 1] Rock
      (`StaticMeshComponent.SetStaticMesh` _pipe_2 "/Game/Runner/Meshes/SM_Rock_Avoid.SM_Rock_Avoid")
      (`SceneComponent.SetWorldScale3D` _pipe_2 (0.9 0.9 0.9))
      (`SceneComponent.K2_SetWorldRotation` :`self` _pipe_2))
    (:`2`
      ;[1 1 1] Table
      (`StaticMeshComponent.SetStaticMesh` _pipe "/Game/Runner/Meshes/SM_TableRound_Avoid.SM_TableRound_Avoid")
      (`SceneComponent.SetWorldScale3D` _pipe (2.0 2.0 2.5))
      (`SceneComponent.K2_SetWorldRotation` _pipe (struct :`Yaw` 90.0) false false))))