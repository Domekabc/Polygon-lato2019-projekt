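; Magnet power-up pickup for the runner that temporarily turns on the player's magnet effect.
; On overlap with the ThirdPersonCharacter it sets MagnetActive, prints a debug message and hides its mesh.
; After a ten-second delay it clears the flag on player character 0 and destroys itself.
; The construction script assigns the Magnet static mesh.
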(event `self.ReceiveActorBeginOverlap`
  (params (OtherActor :type "Actor Object Reference"))
  (bind _asthird_person_character (cast `/Game/ThirdPersonBP/ThirdPersonCharacter` OtherActor))
  (set `/Game/ThirdPersonBP/ThirdPersonCharacter.MagnetActive` true _asthird_person_character)
  (`KismetSystemLibrary.PrintString` "Magnet Active" true true (struct :`R` 1.0 :`G` 0.056108 :`A` 1.0))
  (`SceneComponent.SetVisibility` (`self.StaticMesh`) false false)
  (`KismetSystemLibrary.Delay` 10.0)
  (bind _asthird_person_character_2 (cast `/Game/ThirdPersonBP/ThirdPersonCharacter` (`GameplayStatics.GetPlayerCharacter` 0)))
  (set `/Game/ThirdPersonBP/ThirdPersonCharacter.MagnetActive` false _asthird_person_character_2)
  (`self.K2_DestroyActor`))

(fn `UserConstructionScript`
  (`StaticMeshComponent.SetStaticMesh` (`self.StaticMesh`) "/Game/Runner/Meshes/Magnet.Magnet"))