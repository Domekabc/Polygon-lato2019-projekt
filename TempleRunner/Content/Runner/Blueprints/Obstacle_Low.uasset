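; Low obstacle for a runner game that kills the player character on contact.
; The construction script randomly gives the Pipe mesh component one of three looks (couch, pipes or corner frame), setting world scale and rotation for the latter two.
; On actor overlap it casts to ThirdPersonCharacter and, if not already dead, sets the death flag and calls the character's DeathFunction.
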(event `self.ReceiveActorBeginOverlap`
  (params (OtherActor :type "Actor Object Reference"))
  (bind _asthird_person_character (cast `/Game/ThirdPersonBP/ThirdPersonCharacter` OtherActor))
  (if (not (`/Game/ThirdPersonBP/ThirdPersonCharacter.ISDead` _asthird_person_character))
    (set `/Game/ThirdPersonBP/ThirdPersonCharacter.ISDead` true _asthird_person_character)
    (`/Game/ThirdPersonBP/ThirdPersonCharacter.DeathFunction` _asthird_person_character)))

(fn `UserConstructionScript`
  (bind _pipe (`self.Pipe`))
  (bind _pipe_2 (`self.Pipe`))
  (switch `int` (`KismetMathLibrary.RandomInteger` 3)
    (:`0`
      (`StaticMeshComponent.SetStaticMesh` (`self.Pipe`) "/Game/Runner/Meshes/SM_Couch_low.SM_Couch_low"))
    (:`1`
      (`StaticMeshComponent.SetStaticMesh` _pipe_2 "/Game/Runner/Meshes/Low_Obstacles_Pipes.Low_Obstacles_Pipes")
      (`SceneComponent.SetWorldScale3D` _pipe_2 (1.2 1.2 1.2))
      (`SceneComponent.K2_SetWorldRotation` :`self` _pipe_2))
    (:`2`
      (`StaticMeshComponent.SetStaticMesh` _pipe "/Game/Runner/Meshes/SM_CornerFrame_low.SM_CornerFrame_low")
      (`SceneComponent.SetWorldScale3D` _pipe (5.0 7.0 5.0))
      (`SceneComponent.K2_SetWorldRotation` _pipe (struct :`Yaw` 90.0) false false))))