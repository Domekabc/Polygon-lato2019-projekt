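; Obstacle_Pipe is a low obstacle actor for the runner game that kills the player on contact.
; Its construction script randomly gives the Pipe mesh component either a couch or a pipes mesh, scaling up and resetting world rotation only for the pipes.
; On actor overlap it casts the other actor to ThirdPersonCharacter and calls that character's DeathFunction, ignoring anything else.
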(event `self.ReceiveActorBeginOverlap`
  (params (OtherActor :type "Actor Object Reference"))
  (bind _asthird_person_character (cast `/Game/ThirdPersonBP/ThirdPersonCharacter` OtherActor))
  (`/Game/ThirdPersonBP/ThirdPersonCharacter.DeathFunction` _asthird_person_character))

(fn `UserConstructionScript`
  (bind _pipe (`self.Pipe`))
  (switch `int` (`KismetMathLibrary.RandomInteger` 2)
    (:`0`
      (`StaticMeshComponent.SetStaticMesh` (`self.Pipe`) "/Game/Runner/Meshes/SM_Couch_low.SM_Couch_low"))
    (:`1`
      (`StaticMeshComponent.SetStaticMesh` _pipe "/Game/Runner/Meshes/Low_Obstacles_Pipes.Low_Obstacles_Pipes")
      (`SceneComponent.SetWorldScale3D` _pipe (1.2 1.2 1.2))
      (`SceneComponent.K2_SetWorldRotation` _pipe (struct) false false))))