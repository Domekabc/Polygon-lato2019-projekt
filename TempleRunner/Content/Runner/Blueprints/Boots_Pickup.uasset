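; Boots pickup for the runner game that grants the third-person character a temporary higher jump.
; On overlap it flags the jump power-up, plays a sound, raises jump Z velocity to the character's boosted value and hides its mesh.
; After a timed delay it restores the base jump on player 0's character and destroys itself.
; Collision stays active while hidden.
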(event `self.ReceiveActorBeginOverlap`
  (params (OtherActor :type "Actor Object Reference"))
  (bind _asthird_person_character (cast `/Game/ThirdPersonBP/ThirdPersonCharacter` OtherActor))
  (set `/Game/ThirdPersonBP/ThirdPersonCharacter.JumpPowerUpActive` true _asthird_person_character)
  (`GameplayStatics.PlaySoundAtLocation` "/Game/Runner/SFX/Power_Up_Ray-Mike_Koenig-800933783.Power_Up_Ray-Mike_Koenig-800933783" (`self.K2_GetActorLocation` _asthird_person_character) (struct) 1.0 1.0 0.0 null null null)
  (set `CharacterMovementComponent.JumpZVelocity` (`/Game/ThirdPersonBP/ThirdPersonCharacter.JumpDouble` _asthird_person_character) (`Character.CharacterMovement` _asthird_person_character))
  (`SceneComponent.SetVisibility` (`self.StaticMesh`) false false)
  (`KismetSystemLibrary.Delay` 10.0)
  (bind _asthird_person_character_2 (cast `/Game/ThirdPersonBP/ThirdPersonCharacter` (`GameplayStatics.GetPlayerCharacter` 0)))
  (set `/Game/ThirdPersonBP/ThirdPersonCharacter.JumpPowerUpActive` false _asthird_person_character_2)
  (set `CharacterMovementComponent.JumpZVelocity` (`/Game/ThirdPersonBP/ThirdPersonCharacter.JumpBase` _asthird_person_character_2) (`Character.CharacterMovement` _asthird_person_character_2))
  (`self.K2_DestroyActor`))

(fn `UserConstructionScript`
  (`StaticMeshComponent.SetStaticMesh` (`self.StaticMesh`) "/Game/Runner/Meshes/BootsPickup.BootsPickup"))