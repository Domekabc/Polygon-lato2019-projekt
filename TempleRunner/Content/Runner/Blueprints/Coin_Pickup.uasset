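; Coin pickup for the runner that adds to the game mode's coin count and score, plays a sound and destroys itself when its mesh overlaps the player.
; An outer sphere acts as a magnet trigger while the character's MagnetActive is set.
; A timeline then pulls the coin toward the player with VInterpTo plus a Slide offset.
; Magnetized coins self-destruct after a short delay, scoring only through mesh overlap.
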(event `self.Sphere.OnComponentBeginOverlap`
  (params (OverlappedComponent :type "PrimitiveComponent Object Reference") (OtherActor :type "Actor Object Reference") (OtherComp :type "PrimitiveComponent Object Reference") (OtherBodyIndex :type Integer) (bFromSweep :type Boolean) (SweepResult :type "HitResult Structure (by ref)"))
  ;[1 1 1] Coin Magnet
  (bind _asthird_person_character (cast `/Game/ThirdPersonBP/ThirdPersonCharacter` OtherActor))
  (if (`/Game/ThirdPersonBP/ThirdPersonCharacter.MagnetActive` _asthird_person_character)
    (`|ExecutionSequence`
      (:`then_0`
        (cast `/Game/ThirdPersonBP/ThirdPersonGameMode` (`GameplayStatics.GetGameMode`))
        (`KismetSystemLibrary.Delay` 0.5)
        (`self.K2_DestroyActor`))
      (:`then_1`
        (bind (_direction _slide) (`Timeline|Timeline_0`)
          (:`Update`
            (`self.K2_SetActorLocation` (+ _slide (`KismetMathLibrary.VInterpTo` (.location (`self.GetTransform`)) (`self.K2_GetActorLocation` (`GameplayStatics.GetPlayerCharacter` 0)) (`GameplayStatics.GetWorldDeltaSeconds`) 15.0)))))))))

(event `self.StaticMesh.OnComponentBeginOverlap`
  (params (OverlappedComponent :type "PrimitiveComponent Object Reference") (OtherActor :type "Actor Object Reference") (OtherComp :type "PrimitiveComponent Object Reference") (OtherBodyIndex :type Integer) (bFromSweep :type Boolean) (SweepResult :type "HitResult Structure (by ref)"))
  ;[1 1 1] Coin Mesh collision
  (cast `/Game/ThirdPersonBP/ThirdPersonCharacter` OtherActor)
  (bind _asthird_person_game_mode (cast `/Game/ThirdPersonBP/ThirdPersonGameMode` (`GameplayStatics.GetGameMode`)))
  (set `/Game/ThirdPersonBP/ThirdPersonGameMode.Coins` (+ (`/Game/ThirdPersonBP/ThirdPersonGameMode.Coins` _asthird_person_game_mode) 1) _asthird_person_game_mode)
  (set `/Game/ThirdPersonBP/ThirdPersonGameMode.CurrentPoints` (+ (`/Game/ThirdPersonBP/ThirdPersonGameMode.CurrentPoints` _asthird_person_game_mode) (`self.CoinScoreWorth`)) _asthird_person_game_mode)
  (`GameplayStatics.PlaySound2D` "/Game/Runner/SFX/Pickup_SFX.Pickup_SFX" 1.0 1.0 0.0 null null)
  (`self.K2_DestroyActor`))

(fn `UserConstructionScript`
  (`StaticMeshComponent.SetStaticMesh` (`self.StaticMesh`) "/Game/Runner/Meshes/pickup_kineticEnergy.pickup_kineticEnergy"))